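; BP_HigherSlime is a slime platform that bounces any Character overlapping it high into the air.
; On overlap it runs the parent logic, then calls LaunchCharacter with a strong, purely vertical velocity that adds to the character's current velocity.
; A MoveToTarget event snaps the platform mesh to TargetLocation without sweep or interpolation.
; BeginPlay and construction defer to the parent, and Tick is disabled.
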(event Custom|MoveToTarget
  ;[0.15 0.15 0.15 0.5] Move
  (Transformation|SetWorldLocation (Variables|Default|GetPlatformMesh) (Variables|Default|GetTargetLocation) false false))

(event EventBeginPlay
  (|CallParentFunction))

(event Collision|EventActorBeginOverlap
  (params (OtherActor :type Actor%20Object%20Reference))
  (|CallParentFunction OtherActor)
  (bind _ascharacter (Utilities|Casting|CastToCharacter OtherActor))
  (Character|LaunchCharacter _ascharacter "0.000000,0.000000,2500.000000" false false))

(event EventTick
  (params (DeltaSeconds :type Float%20%28single-precision%29))
  (|CallParentFunction DeltaSeconds) ; This node is disabled and will not be called.\nDrag off pins to build functionality.
)

(fn ConstructionScript
  (|CallParentFunction))