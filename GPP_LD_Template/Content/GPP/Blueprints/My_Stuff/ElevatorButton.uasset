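; An elevator button actor that opens its linked elevator when the player presses the interact input nearby.
; Box overlap with BP_PlayerCharacter toggles an Interactable flag.
; The actor enables input on itself at BeginPlay and handles raw keyboard and gamepad keys directly.
; An accepted press destroys the Box component and calls OpenTheElevator on ElevatorRef.
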(event OnComponentBeginOverlap(Box)
  (params (OverlappedComponent :type Primitive%20Component%20Object%20Reference) (OtherActor :type Actor%20Object%20Reference) (OtherComp :type Primitive%20Component%20Object%20Reference) (OtherBodyIndex :type Integer) (bFromSweep :type Boolean) (SweepResult :type Hit%20Result%20Structure%20%28by%20ref%29))
  ;[0.15 0.15 0.15 0.5] Overlap
  (Utilities|Casting|CastToBP_PlayerCharacter OtherActor)
  (Variables|Default|SetInteractable true))

(event OnComponentEndOverlap(Box)
  (params (OverlappedComponent :type Primitive%20Component%20Object%20Reference) (OtherActor :type Actor%20Object%20Reference) (OtherComp :type Primitive%20Component%20Object%20Reference) (OtherBodyIndex :type Integer))
  ;[0.15 0.15 0.15 0.5] Overlap
  (Utilities|Casting|CastToBP_PlayerCharacter OtherActor)
  (Variables|Default|SetInteractable false))

(event EventBeginPlay
  (Input|EnableInput (Game|GetPlayerController 0)))

(event Collision|EventActorBeginOverlap
  (params (OtherActor :type Actor%20Object%20Reference)))

(event EventTick
  (params (DeltaSeconds :type Float%20%28single-precision%29)))

(event Input|KeyboardEvents|2
  (params (Key :type Key%20Structure :default "None"))
  (:Pressed
    (if (Variables|Default|GetInteractable)
      (Components|DestroyComponent (Variables|Default|GetBox))
      (Default|OpentheElevator (Variables|Default|GetElevatorRef)))))

(event Input|GamepadEvents|GamepadFaceButtonTop
  (params (Key :type Key%20Structure :default "None"))
  (:Pressed
    (if (Variables|Default|GetInteractable)
      (Components|DestroyComponent (Variables|Default|GetBox))
      (Default|OpentheElevator (Variables|Default|GetElevatorRef)))))

(fn ConstructionScript)