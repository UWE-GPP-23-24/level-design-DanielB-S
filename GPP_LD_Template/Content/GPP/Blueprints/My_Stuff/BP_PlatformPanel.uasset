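; Interactable crane control panel that lets the player activate a referenced platform once.
; InteractionBox overlap with BP_PlayerCharacter toggles CanInteract and a button prompt widget; the gamepad top face button or 2 key triggers it.
; Activation destroys the box, then steps a SystemMessageCrane widget through timed power-rerouting messages, calling ActivatePlatform partway through before removing the widget.
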(event OnComponentBeginOverlap(InteractionBox)
  (params (OverlappedComponent :type Primitive%20Component%20Object%20Reference) (OtherActor :type Actor%20Object%20Reference) (OtherComp :type Primitive%20Component%20Object%20Reference) (OtherBodyIndex :type Integer) (bFromSweep :type Boolean) (SweepResult :type Hit%20Result%20Structure%20%28by%20ref%29))
  ;[0.15 0 0.1273 0.5] Checks for Player Overlap with Collider
  (Utilities|Casting|CastToBP_PlayerCharacter OtherActor)
  (Variables|Default|SetCanInteract true)
  (UserInterface|Viewport|AddtoViewport (Variables|Default|GetCraneButton) 0))

(event OnComponentEndOverlap(InteractionBox)
  (params (OverlappedComponent :type Primitive%20Component%20Object%20Reference) (OtherActor :type Actor%20Object%20Reference) (OtherComp :type Primitive%20Component%20Object%20Reference) (OtherBodyIndex :type Integer))
  ;[0.15 0 0.1273 0.5] Checks for Player Overlap with Collider
  (Utilities|Casting|CastToBP_PlayerCharacter OtherActor)
  (Variables|Default|SetCanInteract false)
  (Widget|RemovefromParent (Variables|Default|GetCraneButton)))

(event EventBeginPlay
  ;[0.15 0.1451 0.00679 0.5] Enable Input
  (bind _returnvalue (UserInterface|CreateWidget "/Game/GPP/Blueprints/My_Stuff/PlatformPanelPrompt.PlatformPanelPrompt_C"))
  (Variables|Default|SetCraneButton _returnvalue)
  (Input|EnableInput (Game|GetPlayerController 0)))

(event Collision|EventActorBeginOverlap
  (params (OtherActor :type Actor%20Object%20Reference)))

(event EventTick
  (params (DeltaSeconds :type Float%20%28single-precision%29)))

(event Input|KeyboardEvents|2
  (params (Key :type Key%20Structure :default "None"))
  ;[0.03749 0.1172 0.15 0.5] Keypress to Activate Button
  (:Pressed
    (if (Variables|Default|GetCanInteract)
      (Components|DestroyComponent (Variables|Default|GetInteraction%20Box))
      ;[0.15 0 0 0.5] Create Widget for System UI
      (bind _returnvalue (UserInterface|CreateWidget "/Game/GPP/Blueprints/My_Stuff/SystemMessageCrane.SystemMessageCrane_C"))
      (bind _output_get (Variables|Default|SetTypewriter _returnvalue))
      (UserInterface|Viewport|AddtoViewport _output_get 0)
      ;[0.005409 0.15 0 0.5] Update UI Text
      (Default|UpdateText (Variables|Default|GetTypewriter) "SYSTEM MESSAGE: Crane System Engaged")
      (Utilities|FlowControl|Delay 2.0)
      (Default|UpdateText (Variables|Default|GetTypewriter) "SYSTEM ERROR: Insufficent Power to Engage Crane System")
      (Utilities|FlowControl|Delay 2.0)
      (Default|UpdateText (Variables|Default|GetTypewriter) "SYSTEM MESSAGE: Rerouting Power From Non Essential Systems")
      (Utilities|FlowControl|Delay 2.0)
      (Default|UpdateText (Variables|Default|GetTypewriter) "SYSTEM MESSAGE: Crane System Engaged")
      ;;[0.1416 0 0.15 0.5] Move Platform
      (Default|ActivatePlatform (Variables|Default|GetPlatformReference))
      (Utilities|FlowControl|Delay 2.0)
      (Default|UpdateText (Variables|Default|GetTypewriter) "SYSTEM WARNING: Back-Up Generators Engaged")
      (Utilities|FlowControl|Delay 1.5)
      (Widget|RemovefromParent (Variables|Default|GetTypewriter)))))

(event Input|GamepadEvents|GamepadFaceButtonTop
  (params (Key :type Key%20Structure :default "None"))
  ;[0.03749 0.1172 0.15 0.5] Keypress to Activate Button
  (:Pressed
    (if (Variables|Default|GetCanInteract)
      (Components|DestroyComponent (Variables|Default|GetInteraction%20Box))
      ;[0.15 0 0 0.5] Create Widget for System UI
      (bind _returnvalue (UserInterface|CreateWidget "/Game/GPP/Blueprints/My_Stuff/SystemMessageCrane.SystemMessageCrane_C"))
      (bind _output_get (Variables|Default|SetTypewriter _returnvalue))
      (UserInterface|Viewport|AddtoViewport _output_get 0)
      ;[0.005409 0.15 0 0.5] Update UI Text
      (Default|UpdateText (Variables|Default|GetTypewriter) "SYSTEM MESSAGE: Crane System Engaged")
      (Utilities|FlowControl|Delay 2.0)
      (Default|UpdateText (Variables|Default|GetTypewriter) "SYSTEM ERROR: Insufficent Power to Engage Crane System")
      (Utilities|FlowControl|Delay 2.0)
      (Default|UpdateText (Variables|Default|GetTypewriter) "SYSTEM MESSAGE: Rerouting Power From Non Essential Systems")
      (Utilities|FlowControl|Delay 2.0)
      (Default|UpdateText (Variables|Default|GetTypewriter) "SYSTEM MESSAGE: Crane System Engaged")
      ;;[0.1416 0 0.15 0.5] Move Platform
      (Default|ActivatePlatform (Variables|Default|GetPlatformReference))
      (Utilities|FlowControl|Delay 2.0)
      (Default|UpdateText (Variables|Default|GetTypewriter) "SYSTEM WARNING: Back-Up Generators Engaged")
      (Utilities|FlowControl|Delay 1.5)
      (Widget|RemovefromParent (Variables|Default|GetTypewriter)))))

(fn ConstructionScript)